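; Game instance for a tank game that relays connection, zone list and account events to the UI.
; On connect it queries the zone list, and before joining a game it shows a loading widget.
; Received zone and account data are stored, then pushed to the first top-level MainMenuTest widget if one exists.
; Account updates also write the Cup value to the "cup" leaderboard stat for the first player controller.
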(event EventOnPreJoinGame
  (bind _returnvalue (UserInterface|CreateWidget "/Game/Widget/UI_Loading.UI_Loading_C" (Game|GetPlayerController 0)))
  (UserInterface|Viewport|AddtoViewport _returnvalue 0))

(event EventOnReceiveZoneList
  (params (zoneList :type Array%20of%20Server%20Zone%20Object%20References))
  (Variables|Default|SetZoneList zoneList)
  (bind _foundwidgets (Widget|GetAllWidgetsOfClass "/Game/Widget/MainMenuTest.MainMenuTest_C" true))
  (if (> (Utilities|Array|Length _foundwidgets) 0)
    (Default|UpdateZoneList (Utilities|Array|Get(acopy) _foundwidgets) (Variables|Default|GetZoneList))))

(event EventOnReceiveAccountData
  (params (accountData :type Account%20Data%20Object%20Reference))
  (bind _output_get (Variables|Default|SetAccountData accountData))
  (Class|LeaderboardBlueprintLibrary|WriteLeaderboardInteger (Game|GetPlayerController 0) "cup" (Variables|/Script/OnlineSubsystemEZOnline.AccountData|Getcup _output_get))
  (bind _foundwidgets (Widget|GetAllWidgetsOfClass "/Game/Widget/MainMenuTest.MainMenuTest_C" true))
  (if (> (Utilities|Array|Length _foundwidgets) 0)
    (Default|UpdateAccountData (Utilities|Array|Get(acopy) _foundwidgets) (Variables|Default|GetAccountData))))

(event EventOnConnectComplete
  (Class|EZOnlineGameInstance|QueryZoneList))