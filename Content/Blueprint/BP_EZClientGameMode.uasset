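; Client game mode that shows network status UI while the game connects over a socket.
; On BeginPlay it displays a waiting-for-network widget, and the socket connected event sets a connected flag.
; Socket close or connect failure raises a network error widget and removes the waiting widget.
; Separate events change the waiting text to a Chinese "waiting for login" message or dismiss that widget.
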(event Custom|NetWorkError
  (bind _waitingwidget (Variables|Default|GetWaitingWidget))
  (bind _returnvalue (UserInterface|CreateWidget "/Game/Widget/UI_NetWorkError.UI_NetWorkError_C" (Game|GetPlayerController 0)))
  (UserInterface|Viewport|AddtoViewport _returnvalue 0)
  (Utilities|IsValid _waitingwidget
    (:Is%20Valid
      (Widget|RemovefromParent _waitingwidget))))

(event Custom|RemoveWaiting
  (bind _waitingwidget (Variables|Default|GetWaitingWidget))
  (Utilities|IsValid _waitingwidget
    (:Is%20Valid
      (Widget|RemovefromParent _waitingwidget))))

(event Custom|WaitingLogin
  (bind _waitingwidget (Variables|Default|GetWaitingWidget))
  (Utilities|IsValid _waitingwidget
    (:Is%20Valid
      (Rendering|Components|TextRender|SetText (Variables|/Game/Widget/UI_WaitingNetwork.UI_WaitingNetwork_C|GetShowText _waitingwidget) "等待登陆..."))))

(event EventBeginPlay
  (bind _returnvalue (UserInterface|CreateWidget "/Game/Widget/UI_WaitingNetwork.UI_WaitingNetwork_C" (Game|GetPlayerController 0)))
  (Variables|Default|SetWaitingWidget _returnvalue)
  (UserInterface|Viewport|AddtoViewport _returnvalue 10))

(event EventTick
  (params (DeltaSeconds :type Float%20%28single-precision%29)))

(event EventK2onSocketClosed
  (CallFunction|NetWorkError))

(event EventK2onSocketConnected
  (Variables|Default|SetIsConnected true))

(event EventK2onSocketConnectFail
  (CallFunction|NetWorkError))

(fn ConstructionScript)