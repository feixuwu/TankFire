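; BP_TankBullet is the tank projectile actor, handling the sound and visual effects for its firing and explosion.
; On BeginPlay it spawns an AudioPlayer actor with the firing sound at its own transform.
; When destroyed, it spawns another AudioPlayer for the explosion sound and, on every platform except HTML5, a half-scale, short-lived ParticlePlayer explosion.
; The graph contains no movement or damage logic.
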(event EventBeginPlay
  (Game|SpawnActorfromClass "/Game/Blueprint/AudioPlayer.AudioPlayer_C" (Transformation|GetActorTransform) "AlwaysSpawn" 0 "/Game/StarterContent/Audio/ShotFiring.ShotFiring" 0))

(event EventDestroyed
  (bind _returnvalue (Transformation|GetActorTransform))
  (bind (_location _rotation) (Math|Transform|BreakTransform _returnvalue))
  (Game|SpawnActorfromClass "/Game/Blueprint/AudioPlayer.AudioPlayer_C" _returnvalue "AlwaysSpawn" 0 "/Game/StarterContent/Audio/Explosion01.Explosion01" 0)
  (bind _returnvalue_2 (Game|GetPlatformName))
  (if (Utilities|Enum|NotEqual(Enum) _returnvalue_2 "HTML5")
    (Game|SpawnActorfromClass "/Game/Blueprint/ParticlePlayer.ParticlePlayer_C" (Math|Transform|MakeTransform _location _rotation "0.500000,0.500000,0.500000") "Undefined" 0 "/Game/StarterContent/Particles/P_Explosion.P_Explosion" 1.0 0)))

(event EventTick
  (params (DeltaSeconds :type Float%20%28single-precision%29)))

(fn ConstructionScript)