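; TestTankGameMode is a game mode Blueprint that runs a timed tank match.
; The first player restart starts the match, and Tick counts down the time left stored on TankGameState.
; At zero it processes results with the TankSegmentConf table, finishes the game, then requests application exit after a short delay.
; A disconnected chain for spawning an AI tank and restarting its controller never runs.
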(event EventTick
  (params (DeltaSeconds :type Float%20%28single-precision%29))
  (bind _self self)
  (if (Variables|Default|GetIsGameStarted)
    (bind _astank_game_state (Utilities|Casting|CastToTankGameState (Game|GetGameState)))
    (bind _output_get (Variables|/Script/TankFire.TankGameState|SetGameLeftTime _astank_game_state (- (Variables|/Script/TankFire.TankGameState|GetGameLeftTime _astank_game_state) DeltaSeconds)))
    (if (<= _output_get 0.0)
      (Variables|/Script/TankFire.TankGameState|SetGameLeftTime _astank_game_state 0.0)
      (Class|TankBlueprintLibrary|ProcessGameResult self "/Game/Blueprint/TankSegmentConf.TankSegmentConf")
      (Variables|Default|SetIsGameStarted false)
      (Variables|Default|SetgameFinish true)
      (Class|TankBlueprintLibrary|FinishGame _self)
      (Utilities|FlowControl|Delay 1e+01)
      (Class|EZOnlineFunctionLibrary|RequestExit _self false))))

(event EventOnRestartPlayer
  (params (NewPlayer :type Controller%20Object%20Reference))
  (if (not (Variables|Default|GetIsGameStarted))
    (if (not (Variables|Default|GetgameFinish))
      (Variables|Default|SetIsGameStarted true))))

(fn ConstructionScript)