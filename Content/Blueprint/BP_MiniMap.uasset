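; BP_MiniMap is the minimap scene-capture actor for a tank game, inactive on dedicated servers.
; At BeginPlay it limits the capture to a show-only list of static mesh actors and the sky sphere.
; On throttled timers in Tick, it follows the player pawn in XY and projects every BP_Tank into capture space.
; Those points refill the GameInstance's MapPointList, flagging any tank not controlled by the local player as enemy.
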(event Custom|CacheMapPoint
  (params (DeltaTime :type Float%20%28single-precision%29))
  (bind _output_get (Variables|Default|SetcacheTime (- (Variables|Default|GetcacheTime) DeltaTime)))
  (if (< _output_get 0.0)
    (Variables|Default|SetcacheTime 0.5)
    (bind _astank_game_instance (Utilities|Casting|CastToTankGameInstance (Game|GetGameInstance)))
    (Utilities|Array|Clear (Variables|/Game/Blueprint/TankGameInstance.TankGameInstance_C|GetMapPointList _astank_game_instance))
    (bind _outactors (Actor|GetAllActorsOfClass "/Game/Blueprint/BP_Tank.BP_Tank_C"))
    (for _array_element _outactors
      (bind (_screenpos _returnvalue) (Class|TankBlueprintLibrary|ProjectSceneCapturePosition (Variables|DecalActor|GetCaptureComponent2D) (Transformation|GetActorLocation _array_element)))
      (if _returnvalue
        (Utilities|Array|Add (Variables|/Game/Blueprint/TankGameInstance.TankGameInstance_C|GetMapPointList _astank_game_instance) (Utilities|Struct|MakeMinimapPoint _screenpos (not (== (Pawn|GetController _array_element) (Game|GetPlayerController 0)))))))))

(event Custom|SyncPos
  (params (deltaTime :type Float%20%28single-precision%29))
  (bind _returnvalue (Game|Player|GetPlayerPawn 0))
  (bind _returnvalue_2 (Transformation|GetActorLocation _returnvalue))
  (bind (_x _y) (Math|Vector|BreakVector _returnvalue_2))
  (Utilities|IsValid _returnvalue
    (:Is%20Valid
      (Variables|Default|SetCaptureTime (- (Variables|Default|GetCaptureTime) deltaTime))
      (if (<= (- (Variables|Default|GetCaptureTime) deltaTime) 0.0)
        (Variables|Default|SetCaptureTime 0.5)
        (Transformation|SetActorLocation (Math|Vector|MakeVector _x _y (.Z (Math|Vector|BreakVector (Transformation|GetActorLocation)))) false false)))))

(event EventBeginPlay
  (bind _capturecomponent2d (Variables|DecalActor|GetCaptureComponent2D))
  (if (not (Networking|IsDedicatedServer))
    (bind _outactors (Actor|GetAllActorsOfClass "/Script/Engine.StaticMeshActor"))
    (Variables|Default|SetRenderList _outactors)
    (bind _outactors_2 (Actor|GetAllActorsOfClass "/Engine/EngineSky/BP_Sky_Sphere.BP_Sky_Sphere_C"))
    (Utilities|Array|Add (Variables|Default|GetRenderList) (Utilities|Array|Get(acopy) _outactors_2))
    (Variables|/Script/Engine.SceneCaptureComponent|SetShowOnlyActors _capturecomponent2d (Variables|Default|GetRenderList))
    (Variables|/Script/Engine.SceneCaptureComponent|SetPrimitiveRenderMode _capturecomponent2d "PRM_UseShowOnlyList")))

(event EventTick
  (params (DeltaSeconds :type Float%20%28single-precision%29))
  (if (not (Networking|IsDedicatedServer))
    (CallFunction|SyncPos DeltaSeconds)
    (CallFunction|CacheMapPoint DeltaSeconds)))

(fn ConstructionScript)