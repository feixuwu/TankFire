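; KnockoutTank is a short-lived tank body that gets launched when knocked out, tumbles, then explodes.
; BeginPlay tints both meshes through a dynamic material, feeds HitSpeed to projectile movement and derives a spin rotation from the velocity direction.
; Tick applies that spin until the actor destroys itself after a brief delay.
; Destruction spawns explosion audio except on dedicated servers, plus particles on non-HTML5 platforms.
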(event Custom|SetColor
  (bind _returnvalue (Rendering|Material|CreateDynamicMaterialInstance "/Game/Mesh/Mat/TankMat.TankMat" :!class /Script/Engine.KismetMaterialLibrary))
  (bind _output_get (Variables|Default|SetMatInstance _returnvalue))
  (Rendering|Material|SetVectorParameterValue _output_get "BodyColor" (Variables|Default|GetColor) :!class /Script/Engine.MaterialInstanceDynamic)
  (Rendering|Material|SetMaterial (Variables|Default|GetStaticMesh) 0 (Variables|Default|GetMatInstance))
  (Rendering|Material|SetMaterial (Variables|Default|GetStaticMesh1) 0 (Variables|Default|GetMatInstance)))

(event EventBeginPlay
  (CallFunction|SetColor)
  (Variables|/Script/Engine.MovementComponent|SetVelocity (Variables|Default|GetProjectileMovement) (Variables|Default|GetHitSpeed))
  (Variables|Default|SetTurnRot (Math|Rotator|MakeRotfromZ (Math|Vector|Normalize (Transformation|GetVelocity))))
  (Utilities|FlowControl|Delay 0.4)
  (Actor|DestroyActor))

(event EventDestroyed
  (bind _returnvalue (Transformation|GetActorTransform))
  (if (not (Networking|IsDedicatedServer))
    (Game|SpawnActorfromClass "/Game/Blueprint/AudioPlayer.AudioPlayer_C" _returnvalue "Undefined" 0 "/Game/StarterContent/Audio/TankExplosion.TankExplosion" 0)
    (bind _returnvalue_2 (Game|GetPlatformName))
    (if (Utilities|Enum|NotEqual(Enum) _returnvalue_2 "HTML5")
      (Game|SpawnActorfromClass "/Game/Blueprint/ParticlePlayer.ParticlePlayer_C" (Math|Transform|MakeTransform (.Location (Math|Transform|BreakTransform _returnvalue)) "0, 0, 0" "3.000000,3.000000,3.000000") "Undefined" 0 "/Game/StarterContent/Particles/P_Explosion.P_Explosion" 2.0 0))))

(event EventTick
  (params (DeltaSeconds :type Float%20%28single-precision%29))
  (Transformation|SetActorRotation (Math|Rotator|CombineRotators (Transformation|GetActorRotation) (* (Variables|Default|GetTurnRot) (* DeltaSeconds (Variables|Default|GetTurnSpeed)))) true))

(fn ConstructionScript)