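; Player controller for the tank game that drives match-end, death and kill-notification UI for the player.
; On death it waits a given time, switches to spectator state and shows a death frame with the remaining respawn countdown.
; Kill and killed-by notifications lazily find and cache the GameUI widget, then post a kill message to it.
; Game end adds a GameEnd widget to the viewport.
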(event Custom|SwitchSpectatorCamera
  (params (time :type Float%20%28single-precision%29))
  (Utilities|FlowControl|Delay time)
  (Class|TankPlayerController|ChangetoSpectatorState)
  (bind _returnvalue (UserInterface|CreateWidget "/Game/Widget/UI_DeathFrame.UI_DeathFrame_C" self (- (Variables|Default|GetReliveCountDownTime) time)))
  (UserInterface|Viewport|AddtoViewport _returnvalue 0))

(event Custom|FindUIWidget
  (Utilities|IsValid (Variables|Default|GetGameUIWidget)
    (:Is%20Not%20Valid
      (bind _foundwidgets (Widget|GetAllWidgetsOfClass "/Game/Widget/GameUI.GameUI_C" true))
      (if (> (Utilities|Array|Length _foundwidgets) 0)
        (Variables|Default|SetGameUIWidget (Utilities|Array|Get(acopy) _foundwidgets))))))

(event EventBeginPlay)

(event EventTick
  (params (DeltaSeconds :type Float%20%28single-precision%29)))

(event EventOnGameEnd
  (bind _returnvalue (UserInterface|CreateWidget "/Game/Widget/GameEnd.GameEnd_C" (Game|GetPlayerController 0)))
  (UserInterface|Viewport|AddtoViewport _returnvalue 0))

(event EventNotifyClientbeKilled
  (params (killerName :type String))
  (bind _gameuiwidget (Variables|Default|GetGameUIWidget))
  (CallFunction|FindUIWidget)
  (Utilities|IsValid _gameuiwidget
    (:Is%20Valid
      (bind _asgame_ui (Utilities|Casting|CastToGameUI _gameuiwidget))
      (Default|AddKillMessage _asgame_ui (Utilities|Struct|MakeKillMessage false killerName)))))

(event EventNotifyClientKill
  (params (deathName :type String))
  (bind _gameuiwidget (Variables|Default|GetGameUIWidget))
  (CallFunction|FindUIWidget)
  (Utilities|IsValid _gameuiwidget
    (:Is%20Valid
      (bind _asgame_ui (Utilities|Casting|CastToGameUI _gameuiwidget))
      (Default|AddKillMessage _asgame_ui (Utilities|Struct|MakeKillMessage true deathName)))))

(fn ConstructionScript)