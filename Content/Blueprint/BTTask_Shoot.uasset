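; BTTask_Shoot is a behavior tree task that makes an AI-controlled tank fire at the tank stored in its Target blackboard value.
; It runs a Visibility sphere trace between the two tanks' XY positions, at a height lowered from the target's location, and fails on any hit or invalid target.
; With a clear line, it calls Shoot on the controlled tank with a rotation toward the target and finishes successfully.
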(event EventReceiveExecute
  (params (OwnerActor :type Actor%20Object%20Reference))
  (bind _asaicontroller (Utilities|Casting|CastToAIController OwnerActor)
    (:then
      (bind _asbp_tank (Utilities|Casting|CastToBP_Tank (Class|BTFunctionLibrary|GetBlackboardValueasObject (Variables|Default|GetTarget)))
        (:then
          (Utilities|IsValid _asbp_tank
            (:Is%20Valid
              (bind _returnvalue (Collision|SphereTraceByChannel (Math|Vector|MakeVector (.X (Math|Vector|BreakVector (Transformation|GetActorLocation _asbp_tank))) (.Y (Math|Vector|BreakVector (Transformation|GetActorLocation _asbp_tank))) (- (.Z (Math|Vector|BreakVector (Transformation|GetActorLocation _asbp_tank))) 1.3e+02)) (Math|Vector|MakeVector (.X (Math|Vector|BreakVector (Transformation|GetActorLocation (Pawn|GetControlledPawn _asaicontroller)))) (.Y (Math|Vector|BreakVector (Transformation|GetActorLocation (Pawn|GetControlledPawn _asaicontroller)))) (- (.Z (Math|Vector|BreakVector (Transformation|GetActorLocation _asbp_tank))) 1.3e+02)) 45.0 "TraceTypeQuery1" false 0 "None"))
              (if _returnvalue
                (AI|BehaviorTree|FinishExecute false :!label _label)
                (else
                  (bind _asbp_tank_2 (Utilities|Casting|CastToBP_Tank (Pawn|GetControlledPawn _asaicontroller)))
                  (Class|TankCharacter|Shoot _asbp_tank_2 (Math|Rotator|MakeRotfromX (Math|Vector|Normalize (- (Transformation|GetActorLocation _asbp_tank) (Transformation|GetActorLocation (Pawn|GetControlledPawn _asaicontroller))))))
                  (AI|BehaviorTree|FinishExecute true))))
            (:Is%20Not%20Valid
              (goto _label))))
        (:CastFailed
          (goto _label))))
    (:CastFailed
      (goto _label))))