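; BP_AITankController is the AI controller for computer-driven tanks, giving each a name and starting its behavior.
; On BeginPlay, the server sets the name from a random row of RobotDatatable, with a hardcoded fallback if the lookup fails.
; On possession, also server-only, it sets up AITankBlackboard and runs the BT_AITank behavior tree.
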(event EventBeginPlay
  (Networking|SwitchHasAuthority
    (:Authority
      (bind _outrownames (DataTable|GetDataTableRowNames "/Game/DataTable/RobotDatatable.RobotDatatable"))
      (bind _returnvalue (Utilities|GetDataTableRow "/Game/DataTable/RobotDatatable.RobotDatatable" (Utilities|Array|Get(acopy) _outrownames (Math|Random|RandomInteger (Utilities|Array|Length _outrownames))))
        (:then
          (Class|TankAIController|SetName (Utilities|Struct|BreakRobotConfig _returnvalue)))
        (:RowNotFound
          (Class|TankAIController|SetName "jim"))))))

(event EventOnPossess
  (params (PossessedPawn :type Pawn%20Object%20Reference))
  (Networking|SwitchHasAuthority
    (:Authority
      (Class|AIController|UseBlackboard "/Game/Blueprint/AITankBlackboard.AITankBlackboard")
      (AI|RunBehaviorTree "/Game/Blueprint/BT_AITank.BT_AITank"))))

(fn ConstructionScript)