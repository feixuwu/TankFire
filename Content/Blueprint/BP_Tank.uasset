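; BP_Tank is the player tank pawn, showing its team or player color, invincibility shield and knockout on being hit.
; It reads TankColor and IsInvincible from the player state and binds to their change events, tinting body and gun through a cached dynamic material and attaching a shield particle.
; A hit spawns a KnockoutTank launched along the hit velocity in the same color, then switches the controller to a spectator camera.
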(event Custom|OnInvincibleChg
  (if (Variables|/Script/TankFire.TankPlayerState|GetisInvincible (stale EventOnRepPlayerState _asbp_tank_player_state))
    (Effects|SpawnEmitterAttached "/Game/ParticleSystem/P_Shield.P_Shield" (Variables|Default|GetCapsuleComponent) "None")))

(event Custom|TankColorChg
  (CallFunction|SetTankColor))

(event Custom|SetTankColor
  (Utilities|IsValid (Variables|Default|GetPlayerState)
    (:Is%20Valid
      (Utilities|IsValid (Variables|Default|GetTankMatInstance)
        (:Is%20Valid
          _)
        (:Is%20Not%20Valid
          (bind _returnvalue (Rendering|Material|CreateDynamicMaterialInstance "/Game/Mesh/Mat/TankMat.TankMat" :!class /Script/Engine.KismetMaterialLibrary))
          (Variables|Default|SetTankMatInstance _returnvalue)
          (bind _asbp_tank_player_state (Utilities|Casting|CastToBP_TankPlayerState (Variables|Default|GetPlayerState)))))
      (Rendering|Material|SetVectorParameterValue (Variables|Default|GetTankMatInstance) "BodyColor" (Variables|/Script/TankFire.TankPlayerState|GetTankColor _asbp_tank_player_state) :!class /Script/Engine.MaterialInstanceDynamic)
      (Rendering|Material|SetMaterial (Variables|Default|GetTankBody) 0 (Variables|Default|GetTankMatInstance))
      (Rendering|Material|SetMaterial (Variables|Default|GetTankGun) 0 (Variables|Default|GetTankMatInstance)))))

(event EventBeginPlay
  (CallFunction|SetTankColor))

(event Collision|EventActorBeginOverlap
  (params (OtherActor :type Actor%20Object%20Reference)))

(event EventOnHitwithVelocity
  (params (velocity :type Vector :default "0, 0, 0"))
  (bind _returnvalue (Transformation|GetActorRotation))
  (bind _returnvalue_2 (Pawn|GetController))
  (bind _asbp_tank_player_state (Utilities|Casting|CastToBP_TankPlayerState (Variables|Default|GetPlayerState)))
  (Game|SpawnActorfromClass "/Game/Blueprint/KnockoutTank.KnockoutTank_C" (Math|Transform|MakeTransform (+ (Transformation|GetActorLocation) (* velocity 1e+02)) _returnvalue) "AlwaysSpawn" _returnvalue_2 _returnvalue 6.0 (* velocity (Variables|Default|GetKnckoutSpeed)) (Variables|/Script/TankFire.TankPlayerState|GetTankColor _asbp_tank_player_state) 0)
  (bind _asbp_tank_player_controller (Utilities|Casting|CastToBP_TankPlayerController _returnvalue_2))
  (Default|SwitchSpectatorCamera _asbp_tank_player_controller 0.6))

(event EventPossessed
  (params (NewController :type Controller%20Object%20Reference))
  (if (not (Networking|IsDedicatedServer))
    (bind _astank_player_state (Utilities|Casting|CastToTankPlayerState (Variables|Default|GetPlayerState)))
    (if (Variables|/Script/TankFire.TankPlayerState|GetisInvincible _astank_player_state)
      (Effects|SpawnEmitterAttached "/Game/ParticleSystem/P_Shield.P_Shield" (Variables|Default|GetCapsuleComponent) "None"))))

(event EventTick
  (params (DeltaSeconds :type Float%20%28single-precision%29)))

(event EventOnRepPlayerState
  (CallFunction|SetTankColor)
  (bind _asbp_tank_player_state (Utilities|Casting|CastToBP_TankPlayerState (Variables|Default|GetPlayerState)))
  (EventDispatchers|BindEventtoInvincibleEvent _asbp_tank_player_state (delegate Custom|OnInvincibleChg))
  (EventDispatchers|BindEventtoTankColorChange _asbp_tank_player_state (delegate Custom|TankColorChg))
  (if (Variables|/Script/TankFire.TankPlayerState|GetisInvincible _asbp_tank_player_state)
    (Effects|SpawnEmitterAttached "/Game/ParticleSystem/P_Shield.P_Shield" (Variables|Default|GetCapsuleComponent) "None")))

(fn ConstructionScript)